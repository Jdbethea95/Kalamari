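; Player character that plays eating feedback, shows a win screen at game end, and returns to MenuLevel when it overlaps a BP_Ball.
; BeginPlay binds to OnMunch and OnTimeEnd, which appear to feed Munch and GameEnd.
; Munch briefly fires a Niagara eating effect, then a timeline animates the mesh's Glow material parameter.
; GameEnd adds the WinText widget, disables movement and switches input to UI only.
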(event Custom|Munch
  (bind _ns_eatingsystem (Variables|Default|GetNS_EatingSystem))
  (Components|Activation|Activate _ns_eatingsystem false)
  (Utilities|FlowControl|Delay 0.3)
  (Components|Activation|Deactivate _ns_eatingsystem)
  (bind _glow_intensity (Timeline|Timeline PlayFromStart)
    (:Update
      (Rendering|Material|SetScalarParameterValueonMaterials (Variables|Character|GetMesh) "Glow" _glow_intensity))))

(event Custom|GameEnd
  (bind _returnvalue (UserInterface|CreateWidget "/Game/StarterContent/Developers/Jacob/Ui/WinText.WinText_C"))
  (UserInterface|Viewport|AddtoViewport _returnvalue 0)
  (Pawn|Components|CharacterMovement|DisableMovement (Variables|Character|GetCharacterMovement))
  (Input|SetInputModeUIOnly (Game|GetPlayerController 0) _returnvalue "LockInFullscreen" false))

(event EventBeginPlay
  (EventDispatchers|BindEventtoOnMunch (EventDispatchers|CreateEvent :!event Custom|Munch))
  (EventDispatchers|BindEventtoOnTimeEnd (EventDispatchers|CreateEvent :!event Custom|GameEnd)))

(event Collision|EventActorBeginOverlap
  (params (OtherActor :type Actor%20Object%20Reference))
  (Utilities|Casting|CastToBP_Ball OtherActor
    (:then
      (Game|OpenLevel(byName) "MenuLevel"))
    (:CastFailed
      (Development|PrintText "Failed"))))

(event EventTick
  (params (DeltaSeconds :type Float%20%28single-precision%29)))

(fn ConstructionScript)