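; BP_Ball is a physics-driven ball enemy that chases the player, with a running chef mesh riding above it.
; Each tick it targets the next navigation path point, falling back to the player's location.
; Chase applies impulses that brake off-target motion and ease acceleration between MinAccel and MaxAccel, pushing harder when heading away.
; The chef mesh follows the sphere and faces its horizontal velocity; player overlap only prints a debug message.
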(event OnComponentBeginOverlap(Collider)
  (params (OverlappedComponent :type Primitive%20Component%20Object%20Reference) (OtherActor :type Actor%20Object%20Reference) (OtherComp :type Primitive%20Component%20Object%20Reference) (OtherBodyIndex :type Integer) (bFromSweep :type Boolean) (SweepResult :type Hit%20Result%20Structure%20%28by%20ref%29))
  (Utilities|Casting|CastToBP_Player OtherActor)
  (Development|PrintString "Hello"))

(event Custom|GetPathTarget
  (bind _returnvalue (Class|NavigationSystemV1|FindPathtoActorSynchronously (Transformation|GetWorldLocation (Variables|Default|GetSphere)) (Game|Player|GetPlayerPawn 0) 0.0 (Game|Player|GetPlayerPawn 0) 0))
  (if (>= (Utilities|Array|Length (Variables|/Script/NavigationSystem.NavigationPath|GetPathPoints _returnvalue)) 2)
    (Variables|Default|SetChaseTarget (Utilities|Array|Get(acopy) (Variables|/Script/NavigationSystem.NavigationPath|GetPathPoints _returnvalue) 1))
    (else
      (Variables|Default|SetChaseTarget (Transformation|GetActorLocation (Game|Player|GetPlayerPawn 0))))))

(event Custom|Chase
  (bind _chasetarget (Variables|Default|GetChaseTarget))
  (bind _sphere (Variables|Default|GetSphere))
  (bind _returnvalue (Transformation|GetComponentVelocity _sphere))
  (bind _returnvalue_2 (Transformation|GetWorldLocation _sphere))
  (bind _returnvalue_3 (Math|Vector|GetUnitDirection(Vector) _returnvalue_2 _chasetarget))
  (bind _returnvalue_4 (Math|Vector|Distance(Vector) _returnvalue "0, 0, 0"))
  (bind _returnvalue_5 (Math|Vector|Normalize _returnvalue))
  (bind _returnvalue_6 (Math|Vector|DotProduct _returnvalue_3 _returnvalue_5))
  (Physics|AddImpulse (Variables|Default|GetSphere) (+ (* (* _returnvalue -1.0) (* (- 1.0 (Math|Float|Absolute(Float) _returnvalue_6)) 2.0)) (* _returnvalue_3 (Math|Interpolation|Ease "ExpoOut" (+ (* _returnvalue_6 -0.5) 0.5) (Variables|Default|GetMinAccel) (Variables|Default|GetMaxAccel)))) "None" false)
  (Variables|Default|SetVelocity _returnvalue_4)
  (Utilities|String|LogString (Utilities|String|ToString(Float) _returnvalue_4)))

(event Custom|ChasePlayer
  (Variables|Default|SetChaseTarget (Transformation|GetActorLocation (Game|Player|GetPlayerPawn 0)))
  (CallFunction|Chase))

(event EventBeginPlay)

(event Collision|EventActorBeginOverlap
  (params (OtherActor :type Actor%20Object%20Reference)))

(event EventTick
  (params (DeltaSeconds :type Float%20%28single-precision%29))
  (bind _sphere (Variables|Default|GetSphere))
  (CallFunction|GetPathTarget)
  (CallFunction|Chase)
  (Transformation|SetWorldLocationAndRotation (Variables|Default|GetCheffRunning) (+ (Transformation|GetWorldLocation _sphere) "0.000000,0.000000,70.000000") (Math|Rotator|MakeRotfromX (* (Transformation|GetComponentVelocity _sphere) "1.000000,1.000000,0.000000")) false false)
  (Transformation|AddWorldRotation (Variables|Default|GetCheffRunning) "0.000000,90.000000,0.000000" false false))

(fn ConstructionScript)